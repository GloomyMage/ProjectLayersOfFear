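; BP_Door is a door the player swings by holding the interact input and turning in first person.
; On press, a debug-drawn camera line trace checks whether any BP_Door is within range.
; While held, Tick rotates the door by the character's TurnRate times Sensitivity.
; A ClampAngle check on world yaw detects the open limits and resets relative yaw just inside them, with debug prints throughout.
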(event Input|EnhancedActionEvents|EnhancedInputActionIA_Interact
  (params (ActionValue :type Boolean) (ElapsedSeconds :type Float%20%28double-precision%29) (TriggeredSeconds :type Float%20%28double-precision%29) (InputAction :type Input%20Action%20Object%20Reference :default "/Game/FirstPerson/Input/Actions/IA_Interact.IA_Interact"))
  (:Started
    (Variables|Default|SetIsHoldingLMB true)
    (bind _asbp_first_person_character (Utilities|Casting|CastToBP_FirstPersonCharacter (Game|GetPlayerCharacter 0)))
    (bind (_outhit _returnvalue) (Collision|LineTraceForObjects (Transformation|GetWorldLocation (Variables|/Game/FirstPerson/Blueprints/BP_FirstPersonCharacter.BP_FirstPersonCharacter_C|GetFirstPersonCamera _asbp_first_person_character)) (+ (Transformation|GetWorldLocation (Variables|/Game/FirstPerson/Blueprints/BP_FirstPersonCharacter.BP_FirstPersonCharacter_C|GetFirstPersonCamera _asbp_first_person_character)) (* (Math|Vector|GetForwardVector (Variables|/Game/FirstPerson/Blueprints/BP_FirstPersonCharacter.BP_FirstPersonCharacter_C|GetFirstPersonCamera _asbp_first_person_character)) (Variables|Default|GetMaxDistance))) (Utilities|Array|MakeArray "ObjectTypeQuery2") false 0 "ForDuration" false))
    (if _returnvalue
      (Utilities|Casting|CastToBP_Door (.HitActor (Collision|BreakHitResult _outhit)))
      (Variables|Default|SetIsLookingAtDoor true)
      (else
        (Variables|Default|SetIsLookingAtDoor false))))
  (:Completed
    (Variables|Default|SetIsHoldingLMB false)))

(event EventBeginPlay
  ;[1 1 1] Enable Use of LMB
  (Input|EnableInput (Game|GetPlayerController 0)))

(event EventTick
  (params (DeltaSeconds :type Float%20%28single-precision%29))
  (bind _open_angle (Variables|Default|GetOpen%20Angle))
  (bind _door (Variables|Default|GetDoor))
  (bind _door_2 (Variables|Default|GetDoor))
  (bind _returnvalue (Transformation|GetWorldRotation _door))
  (if (Variables|Default|GetIsHoldingLMB)
    (Development|PrintString "Hello")
    (if (Variables|Default|GetIsLookingAtDoor)
      (Development|PrintString "Yo")
      (if (not (== (.yaw _returnvalue) (Math|Float|ClampAngle (.yaw _returnvalue) _open_angle (* _open_angle -1.0))))
        (Development|PrintString "A")
        (Transformation|AddLocalRotation _door_2 (Math|Rotator|MakeRotator 0.0 0.0 (* (Variables|/Game/FirstPerson/Blueprints/BP_FirstPersonCharacter.BP_FirstPersonCharacter_C|GetTurn%20Rate (stale Input|EnhancedActionEvents|EnhancedInputActionIA_Interact _asbp_first_person_character)) (Variables|Default|GetSensitivity))) false false)
        (else
          (Development|PrintString "B")
          (if (>= (.yaw _returnvalue) _open_angle)
            (Transformation|SetRelativeRotation _door_2 (Math|Rotator|MakeRotator 0.0 0.0 (- _open_angle 1.0)) false false)
            (else
              (Transformation|SetRelativeRotation _door_2 (Math|Rotator|MakeRotator 0.0 0.0 (+ (* _open_angle -1.0) 1.0)) false false))))))))

(fn ConstructionScript)